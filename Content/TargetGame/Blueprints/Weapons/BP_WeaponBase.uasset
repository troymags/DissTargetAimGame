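; Base weapon Blueprint that handles magazine ammo, firing and timed reloading, with an empty TraceWeapon event as the hit-logic hook.
; FireWeapon spends a round, spawns the fire emitter at the Arrow component and calls TraceWeapon, triggering a reload when ammo runs out.
; ReloadWeapon and Reload share one Delay that refills the magazine.
; The fire sound node is unconnected, and GetFOVMultiplier is a stub returning zero.
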(event Custom|ReloadWeapon
  ;[1 0 0] Reload - May not include
  (Utilities|FlowControl|Delay (Variables|Ammo|GetReloadTime))
  (Variables|Ammo|SetAmmo (Variables|Ammo|GetMaxAmmoMag)))

(event Custom|TraceWeapon)

(event EventFireWeapon
  (Utilities|INT<=INT (Variables|Ammo|GetAmmo)
    (:True
      (CallFunction|ReloadWeapon))
    (:False
      (Variables|Ammo|SetAmmo (- (Variables|Ammo|GetAmmo) 1))
      (CallFunction|WeaponFIreEffect)
      (CallFunction|TraceWeapon)
      (Utilities|INT<=INT (Variables|Ammo|GetAmmo)
        (:True
          (CallFunction|ReloadWeapon))))))

(event EventReload
  ;[1 0 0] Reload - May not include
  (Utilities|FlowControl|Delay (Variables|Ammo|GetReloadTime))
  (Variables|Ammo|SetAmmo (Variables|Ammo|GetMaxAmmoMag)))

(event EventBeginPlay
  (Variables|Ammo|SetAmmo (Variables|Ammo|GetMaxAmmoMag)))

(fn ConstructionScript)

(fn WeaponFIreEffect
  (bind _arrow (Variables|Default|GetArrow))
  (bind _returnvalue (Transformation|GetWorldTransform _arrow))
  (Effects|SpawnEmitteratLocation (Variables|WeaponFireEffects|GetWeaponFireEmitter) (.location _returnvalue) (.rotation _returnvalue) (Variables|WeaponFireEffects|GetWeaponFireEmitterScale))
  (return))

(fn GetFOVMultiplier
  (return 0.0))