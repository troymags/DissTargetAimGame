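; BP_Target is a target actor that randomizes its size and one of several behaviours in the Construction Script.
; On BeginPlay it runs the behaviour: horizontal or vertical movement by a random distance, or a scale pulse up to 1.5 times its size.
; A single timeline, T_Movement, drives all three motions by lerping the SMTarget mesh's relative location or world scale from its Alpha.
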(event EventBeginPlay
  (bind _returnvalue (Math|Random|RandomFloatinRange 75.0 275.0))
  (bind _sm_target (Variables|Default|GetSM_Target))
  (bind _targetscale (Variables|Default|GetTargetScale))
  (bind _returnvalue_2 (* _targetscale 1.5))
  (switch Utilities|FlowControl|Switch|SwitchonE_TargetBehaviour (Variables|Default|GetTargetBehaviour)
    (:NewEnumerator1
      (Variables|Default|SetDestPosition (Math|Vector|MakeVector _returnvalue 0.0 0.0))
      (bind _alpha (Timeline|T_Movement PlayFromStart)
        (:Update
          (switch Utilities|FlowControl|Switch|SwitchonE_TargetBehaviour (Variables|Default|GetTargetBehaviour)
            (:NewEnumerator1
              (Transformation|SetRelativeLocation _sm_target (Math|Vector|Lerp(Vector) "0, 0, 0" (Variables|Default|GetDestPosition) _alpha) false false :!label _label))
            (:NewEnumerator2
              (goto _label))
            (:NewEnumerator3
              (Transformation|SetWorldScale3D _sm_target (Math|Vector|Lerp(Vector) (Math|Vector|MakeVector _targetscale _targetscale _targetscale) (Math|Vector|MakeVector _returnvalue_2 _returnvalue_2 _returnvalue_2) _alpha)))))))
    (:NewEnumerator2
      (Variables|Default|SetDestPosition (Math|Vector|MakeVector 0.0 0.0 _returnvalue))
      (Timeline|T_Movement PlayFromStart))
    (:NewEnumerator3
      (Timeline|T_Movement PlayFromStart))))

(fn ConstructionScript
  (bind _output_get (Variables|Default|SetTargetScale (Math|Random|RandomFloatinRange 0.5 1.5)))
  (Transformation|SetWorldScale3D (Variables|Default|GetSM_Target) (Math|Vector|MakeVector _output_get _output_get _output_get))
  (Variables|Default|SetTargetBehaviour (Utilities|Enum|ByteToEnumE_TargetBehaviour (Math|Conversions|ToByte(Integer) (Math|Random|RandomIntegerinRange 0 3)))))