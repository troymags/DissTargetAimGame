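; Target spawner actor that keeps up to three BP_Target actors in play at random points inside its box volume.
; StartSpawn spawns an initial batch and starts a looping one-second timer that tops up targets whenever the world count drops below the cap.
; Each target spawns rotated toward the player camera with a yaw offset.
; The construction script sizes the spawn box from the BoxExtent variable, and BeginPlay does nothing.
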(event Custom|SpawnTarget
  (bind _spawnarea (Variables|Default|GetSpawnArea))
  ;[0.6399 0.4698 1] Spawn Targets
  (bind _outactors (Actor|GetAllActorsOfClass "/Game/TargetGame/Blueprints/Target/BP_Target.BP_Target_C"))
  (if (<= (Utilities|Array|Length _outactors) 2)
    (bind _output_get (Variables|Default|SetSpawnLocation (Math|Random|RandomPointinBoundingBox (Transformation|GetWorldLocation _spawnarea) (Components|Box|GetScaledBoxExtent _spawnarea))))
    (Game|SpawnActorfromClass "/Game/TargetGame/Blueprints/Target/BP_Target.BP_Target_C" (Math|Transform|MakeTransform _output_get (Math|Rotator|MakeRotator (.roll (Math|Rotator|FindLookatRotation _output_get (Transformation|GetWorldLocation (Variables|/Script/Engine.PlayerCameraManager|GetTransformComponent (Game|GetPlayerCameraManager 0))))) (.pitch (Math|Rotator|FindLookatRotation _output_get (Transformation|GetWorldLocation (Variables|/Script/Engine.PlayerCameraManager|GetTransformComponent (Game|GetPlayerCameraManager 0))))) (- (.yaw (Math|Rotator|FindLookatRotation _output_get (Transformation|GetWorldLocation (Variables|/Script/Engine.PlayerCameraManager|GetTransformComponent (Game|GetPlayerCameraManager 0))))) 9e+01)) "1.000000,1.000000,1.000000") "AdjustIfPossibleButAlwaysSpawn" "MultiplyWithRoot" 0 0)))

(event Custom|StartSpawn
  ;[0.4892 0.9801 1] Start Spawning
  (Utilities|Time|SetTimerbyEvent (delegate Custom|SpawnTarget) 1.0 true)
  (for _index (range 0 2)
    (CallFunction|SpawnTarget)))

(event EventBeginPlay)

(fn ConstructionScript
  (Components|Box|SetBoxExtent (Variables|Default|GetSpawnArea) (Variables|Default|GetBoxExtent) true))